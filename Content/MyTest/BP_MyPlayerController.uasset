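; Player controller that handles sprinting, object interaction and death for BP_MyCharacter.
; On BeginPlay the local controller adds the input mapping, caches the character and creates the UI.
; Sprint swaps walk speed and drives stamina drain and regeneration through a looping Delay.
; A per-tick camera trace highlights BP_Interactable actors for left-click use; touch traces only print, T and O are debug keys, and KillPlayer opens L_MyLevel.
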(event `self.ReceiveBeginPlay`
  (`|ExecutionSequence`
    (:`then_0`
      (switch `string` (`GameplayStatics.GetPlatformName`)))
    (:`then_1`
      (if (`self.IsLocalPlayerController`)
        (`EnhancedInputSubsystemInterface.AddMappingContext` (subsystem `EnhancedInputLocalPlayerSubsystem`) "/Game/MyTest/IMC_MyDefault.IMC_MyDefault" 0 (struct))
        (set `self.PlayerCharacter` (cast `/Game/MyTest/BP_MyCharacter` (`GameplayStatics.GetPlayerCharacter` 0) :!pure true))
        (set `CharacterMovementComponent.MaxWalkSpeed` (`self.WalkSpeed`) (`Character.CharacterMovement` (`self.PlayerCharacter`)))
        (set `self.Stamina` (`self.MaxStamina`))
        (bind _returnvalue (`|CreateWidget` "/Game/MyTest/WBP_MyUI.WBP_MyUI_C"))
        (`UserWidget.AddToPlayerScreen` _returnvalue 0)
        (set `self.SpawnTranform` (`self.GetTransform` (`self.PlayerCharacter`)))))))

(event `EnhancedInput|/Game/MyTest/IA_MySprint`
  (params (ActionValue :type Boolean) (ElapsedSeconds :type "Float (double-precision)") (TriggeredSeconds :type "Float (double-precision)") (InputAction :type "InputAction Object Reference" :default "/Game/MyTest/IA_MySprint.IA_MySprint"))
  (:`Started`
    (set `CharacterMovementComponent.MaxWalkSpeed` (`self.RunSpeed`) (`Character.CharacterMovement` (`self.PlayerCharacter`)))
    (set `self.Walking` false)
    (if (not (and (== (`self.Stamina`) (`self.MaxStamina`)) (`self.Walking`))) :!label _label
      (set `self.Stamina` (+ (`self.Stamina`) (- (* (`KismetMathLibrary.Conv_BoolToInt` (`self.Walking`)) 2) 1)))
      (`KismetSystemLibrary.Delay` 0.01)
      (if (== (`self.Stamina`) 0.0)
        (set `CharacterMovementComponent.MaxWalkSpeed` (`self.WalkSpeed`) (`Character.CharacterMovement` (`self.PlayerCharacter`)) :!label _label_2)
        (set `self.Walking` true)
        (goto _label)
        (else
          (goto _label)))))
  (:`Canceled`
    (goto _label_2))
  (:`Completed`
    (goto _label_2)))

(event `Key|T`
  (params (Key :type "Key Structure"))
  (bind _playercharacter (`self.PlayerCharacter`))
  ; Debug
  (:`Pressed`
    (`/Engine/EditorBlueprintResources/StandardMacros.FlipFlop`
      (:`A`
        (`/Game/MyTest/BP_MyCharacter.HidePlayer` _playercharacter)
        (set `self.IsHiding` true))
      (:`B`
        (`/Game/MyTest/BP_MyCharacter.UnhidePlayer` _playercharacter)
        (set `self.IsHiding` false)))))

(event `Key|O`
  (params (Key :type "Key Structure"))
  ; Debug
  (:`Pressed`
    (`/Game/MyTest/Vampire/Blueprints/BP_Enemy_Base.SetNewDestination` (`self.enemydebug`) null)))

(event `self.ReceiveTick`
  (params (DeltaSeconds :type "Float (single-precision)"))
  (bind _currentinteractable (`self.CurrentInteractable`))
  (bind _returnvalue (`self.K2_GetPawn` (`GameplayStatics.GetPlayerController` 0)))
  ; Interact
  (bind _returnvalue_2 (`BlueprintCameraPoseFunctionLibrary.MakeCameraPoseFromCameraComponent` (`/Game/MyTest/BP_MyCharacter.Camera` (cast `/Game/MyTest/BP_MyCharacter` _returnvalue :!pure true))))
  (bind (_origin _direction) (break `Ray` (`BlueprintCameraPoseFunctionLibrary.GetAimRay` _returnvalue_2)))
  (bind _outhit (`KismetSystemLibrary.LineTraceSingle` _origin (+ _origin (* _direction 500.0)) "TraceTypeQuery2" false (`|MakeArray` _returnvalue :!type "Actor Object Reference")))
  (bind (_asbp_interactable _bsuccess) (cast `/Game/MyTest/Interactables/BP_Interactable` (`.HitActor` (`GameplayStatics.BreakHitResult` _outhit)) :!pure true))
  (if _bsuccess
    (if (`/Game/MyTest/Interactables/BP_Interactable.Interactable` _asbp_interactable)
      (bind _output_get (set `self.CurrentInteractable` _asbp_interactable))
      (`/Game/MyTest/Interactables/BP_Interactable.ShowInteractable` _output_get true))
    (else
      (`/Engine/EditorBlueprintResources/StandardMacros.IsValid` _currentinteractable
        (:`Is Valid`
          (if true
            (`/Game/MyTest/Interactables/BP_Interactable.ShowInteractable` _currentinteractable false)
            (set `self.CurrentInteractable` null :!label _label_3)))
        (:`Is Not Valid`
          (goto _label_3))))))

(event `Key|LeftMouseButton`
  (params (Key :type "Key Structure"))
  (bind _currentinteractable (`self.CurrentInteractable`))
  (:`Pressed`
    (if (not (`/Game/MyTest/BP_MyCharacter.Frozen` (`self.PlayerCharacter`)))
      (`/Engine/EditorBlueprintResources/StandardMacros.IsValid` _currentinteractable
        (:`Is Valid`
          (`/Game/MyTest/Interactables/BP_Interactable.Interaction` _currentinteractable))))))

(event `InputTouch`
  (params (Location :type "Vector Structure") (FingerIndex :type "ETouchIndex Enum"))
  (bind (_worldlocation _worlddirection) (`self.DeprojectScreenPositionToWorld` Location_X Location_Y))
  (:`Pressed`
    (bind _outhit (`KismetSystemLibrary.LineTraceSingle` _worldlocation (+ _worldlocation (* _worlddirection 5000)) "TraceTypeQuery1" false (`|MakeArray` (`self.K2_GetPawn`)) "None" true (struct :`R` 1.0 :`A` 1.0) (struct :`G` 1.0 :`A` 1.0) 0.1))
    (cast `/Game/MyTest/Interactables/BP_Interactable` (`.HitActor` (`GameplayStatics.BreakHitResult` _outhit)))
    (`KismetSystemLibrary.PrintString` "InteractableTouched")))

(fn `KillPlayer`
  (`GameplayStatics.OpenLevelBySoftObjectPtr` "/Game/MyTest/L_MyLevel.L_MyLevel"))

(fn `UserConstructionScript`)