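; Player character that moves and aims through Enhanced Input and can be frozen or hidden.
; Movement follows control yaw, and orient-rotation-to-movement switches off while move input is held, then back on.
; A Frozen flag gates Move and Aim, while hide and unhide functions also toggle visibility and capsule collision.
; A debug F key emits AI noise at the character's location and prints a message.
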(event `EnhancedInput|/Game/MyTest/IA_MyAim`
  (params (ActionValue :type "Vector2D Structure") (ElapsedSeconds :type "Float (double-precision)") (TriggeredSeconds :type "Float (double-precision)") (InputAction :type "InputAction Object Reference" :default "/Game/MyTest/IA_MyAim.IA_MyAim"))
  (:`Triggered`
    (`self.Aim` ActionValue_X ActionValue_Y)))

(event `EnhancedInput|/Game/MyTest/IA_MyMove`
  (params (ActionValue :type "Vector2D Structure") (ElapsedSeconds :type "Float (double-precision)") (TriggeredSeconds :type "Float (double-precision)") (InputAction :type "InputAction Object Reference" :default "/Game/MyTest/IA_MyMove.IA_MyMove"))
  (bind _charactermovement (`self.CharacterMovement`))
  (:`Triggered`
    (`self.Move` ActionValue_X ActionValue_Y))
  (:`Started`
    (set `CharacterMovementComponent.bOrientRotationToMovement` false _charactermovement))
  (:`Canceled`
    (set `CharacterMovementComponent.bOrientRotationToMovement` true _charactermovement :!label _label))
  (:`Completed`
    (goto _label)))

(event `Key|F`
  (params (Key :type "Key Structure"))
  ; Debug
  (:`Pressed`
    (`self.MakeNoise` 100.0 self (`self.K2_GetActorLocation`) 100.0)
    (`KismetSystemLibrary.PrintString` "*Gling !!!")))

(fn `Aim`
  (params (`X Axis` :type "Float (double-precision)") (`Y Axis` :type "Float (double-precision)"))
  (if (not (`self.Frozen`))
    (`self.AddControllerYawInput` `X Axis`)
    (bind _result (`/Engine/EditorBlueprintResources/StandardMacros.NegateFloat` `Y Axis`)
      (:`  `
        (`self.AddControllerPitchInput` _result)))))

(fn `FreezePlayer`
  (set `self.Frozen` true))

(fn `HidePlayer`
  (`self.FreezePlayer`)
  (`self.SetActorHiddenInGame` true)
  (`PrimitiveComponent.SetCollisionEnabled` (`self.CapsuleComponent`) "NoCollision"))

(fn `Move`
  (params (`X Axis` :type "Float (double-precision)") (`Y Axis` :type "Float (double-precision)"))
  (bind (_returnvalue_roll _returnvalue_pitch _returnvalue_yaw) (`KismetMathLibrary.BreakRotator` (`self.GetControlRotation`)))
  (bind (_returnvalue_roll_2 _returnvalue_pitch_2 _returnvalue_yaw_2) (`KismetMathLibrary.BreakRotator` (`self.GetControlRotation`)))
  (if (not (`self.Frozen`))
    (`self.AddMovementInput` (`KismetMathLibrary.GetRightVector` (`KismetMathLibrary.MakeRotator` _returnvalue_roll_2 0.0 _returnvalue_yaw_2)) `X Axis`)
    (`self.AddMovementInput` (`KismetMathLibrary.GetForwardVector` (`KismetMathLibrary.MakeRotator` 0.0 0.0 _returnvalue_yaw)) `Y Axis`)))

(fn `UnfreezePlayer`
  (set `self.Frozen` false))

(fn `UnhidePlayer`
  (`self.UnfreezePlayer`)
  (`self.SetActorHiddenInGame` false)
  (`PrimitiveComponent.SetCollisionEnabled` (`self.CapsuleComponent`) "QueryAndPhysics"))

(fn `UserConstructionScript`)