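; BP_Enemy_Base is the base vampire enemy character, providing a lethal attack and patrol and movement helpers.
; Attack freezes the player character and plays the vampire attack montage, then on completion or interruption has the player controller kill the player and signals the attack's end.
; Getters expose its patrol routes, and SetMovementSpeed maps a movement state from idle to sprinting onto the character's max walk speed.
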(event `Attack`
  (bind _asbp_my_character (cast `/Game/MyTest/BP_MyCharacter` (`GameplayStatics.GetPlayerCharacter` 0) :!pure true))
  (`/Game/MyTest/BP_MyCharacter.FreezePlayer` _asbp_my_character)
  (`|PlayMontage` (`self.Mesh`) "/Game/MyTest/Vampire/AM_Vampire_Attack.AM_Vampire_Attack"
    (:`OnCompleted`
      _)
    (:`OnInterrupted`
      _))
  (`/Engine/EditorBlueprintResources/StandardMacros.IsValid` _asbp_my_character
    (:`Is Valid`
      (`/Game/MyTest/BP_MyPlayerController.KillPlayer` (cast `/Game/MyTest/BP_MyPlayerController` (`self.GetController` _asbp_my_character) :!pure true))
      (`self.OnAttackEnd`))))

(fn `GetPatrolRoute`
  (returns (PatrolRoute :type "/Game/MyTest/Vampire/Blueprints/BP_PatrolRoute Object Reference"))
  (return (`self.PatrolRoute`)))

(fn `GetPatrolRoutes`
  (returns (`Patrol Routes` :type "Array of /Game/MyTest/Vampire/Blueprints/BP_PatrolRoute Object Reference"))
  (return (`self.PatrolRoutes`)))

(fn `SetMovementSpeed`
  (params (MovementSpeed :type "/Game/MyTest/Vampire/Enums/E_MovementSpeed Enum" :default "NewEnumerator0"))
  (returns (SpeedValue :type "Float (double-precision)"))
  (set `CharacterMovementComponent.MaxWalkSpeed` (select `/Game/MyTest/Vampire/Enums/E_MovementSpeed` MovementSpeed :`NewEnumerator1` 100.0 :`NewEnumerator2` 300.0 :`NewEnumerator3` 500.0 :!type "Float (single-precision)") (`self.CharacterMovement`))
  (return 0.0))

(fn `UserConstructionScript`)