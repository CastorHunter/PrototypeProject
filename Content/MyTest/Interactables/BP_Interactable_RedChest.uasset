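; Red chest interactable that gives the player a key, extending a parent interactable Blueprint.
; On interaction it runs the parent logic, disables further interaction and adds the Key to the Items collection on BP_MyPlayerController.
; Its ShowInteractable override calls the parent, then swaps the Cube's material to indicate whether it is interactable.
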(fn `Interaction`
  (`parent.Interaction`)
  (set `self.Interactable` false)
  (`KismetArrayLibrary.Array_Add` (`/Game/MyTest/BP_MyPlayerController.Items` (cast `/Game/MyTest/BP_MyPlayerController` (`GameplayStatics.GetPlayerController` 0) :!pure true)) (`self.Key`)))

(fn `ShowInteractable`
  (params (IsInteractable :type Boolean))
  (`parent.ShowInteractable` IsInteractable)
  (if IsInteractable
    (`PrimitiveComponent.SetMaterial` (`self.Cube`) 0 "/Engine/VREditor/UI/ArrowMaterial.ArrowMaterial")
    (else
      (`PrimitiveComponent.SetMaterial` (`self.Cube`) 0 "/Engine/EngineDebugMaterials/HeatmapMaterial.HeatmapMaterial"))))

(fn `UserConstructionScript`
  (`parent.UserConstructionScript`))