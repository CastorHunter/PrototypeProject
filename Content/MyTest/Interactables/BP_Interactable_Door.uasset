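; Interactable door Blueprint that opens when the player uses it while holding a suitable key.
; Interaction scans the player controller's Items for BP_Key entries: a No Key type opens any door, while Red or Blue must match DoorKeyType.
; Opening disables further interaction and rotates the Billboard; the interactable highlight swaps the Cube's material.
; Shortly after BeginPlay, the whole actor shifts downward.
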(event `self.ReceiveBeginPlay`
  (`KismetSystemLibrary.Delay` 0.1)
  (`self.K2_SetActorLocation` (`KismetMathLibrary.MakeVector` (.x (`self.K2_GetActorLocation`)) (.y (`self.K2_GetActorLocation`)) (- (.z (`self.K2_GetActorLocation`)) 400.0))))

(fn `Interaction`
  (`parent.Interaction`)
  (if (not (`self.Opened`))
    (for _array_element (`/Game/MyTest/BP_MyPlayerController.Items` (cast `/Game/MyTest/BP_MyPlayerController` (`GameplayStatics.GetPlayerController` 0) :!pure true))
      (bind _asbp_key (cast `/Game/MyTest/Items/BP_Key` _array_element))
      (bind _keytype (`/Game/MyTest/Items/BP_Key.KeyType` _asbp_key))
      (switch `/Game/MyTest/Interactables/E_KeyTypes` _keytype
        (:`NewEnumerator0`
          (`self.OpenDoor`))
        (:`NewEnumerator1`
          (if (`|EnumEquality` _keytype (`self.DoorKeyType`)) :!label _label
            (`self.OpenDoor`)))
        (:`NewEnumerator2`
          (goto _label))))))

(fn `OpenDoor`
  (set `self.Interactable` false)
  (set `self.Opened` true)
  (`SceneComponent.K2_SetRelativeRotation` (`self.Billboard`) (struct :`Yaw` 90.0) false false))

(fn `ShowInteractable`
  (params (IsInteractable :type Boolean))
  (`parent.ShowInteractable` IsInteractable)
  (if IsInteractable
    (`PrimitiveComponent.SetMaterial` (`self.Cube`) 0 "/Engine/VREditor/UI/ArrowMaterial.ArrowMaterial")
    (else
      (`PrimitiveComponent.SetMaterial` (`self.Cube`) 0 "/Engine/EngineDebugMaterials/HeatmapMaterial.HeatmapMaterial"))))

(fn `UserConstructionScript`
  (`parent.UserConstructionScript`))